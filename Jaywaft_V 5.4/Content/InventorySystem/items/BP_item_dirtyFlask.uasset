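; BP_item_dirtyFlask is an inventory item for a dirty flask that can be converted into a clean one.
; The createCleanFlask event spawns BP_item_cleanFlask at the player character's location, plays a sound at world origin and destroys the dirty flask.
; GetDropLocation returns a random point within a cone in front of the owner, at a fixed distance.
; The default BeginPlay, overlap and Tick events are disabled.
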(event Custom|createCleanFlask
  (Game|SpawnActorfromClass "/Game/InventorySystem/items/BP_item_cleanFlask.BP_item_cleanFlask_C" (Math|Transform|MakeTransform (Transformation|GetActorLocation (Game|GetPlayerCharacter 0)) "0, 0, 0" "1.000000,1.000000,1.000000") "Undefined" "MultiplyWithRoot" 0 0)
  (Audio|PlaySoundatLocation "/Game/StarterContent/Audio/Light01.Light01" "0, 0, 0" "0, 0, 0" 1.0 1.0 0.0 0 0 0 0)
  (Actor|DestroyActor))

(event EventBeginPlay
  (|CallParentFunction) ; This node is disabled and will not be called.\nDrag off pins to build functionality.
)

(event Collision|EventActorBeginOverlap
  (params (OtherActor :type Actor%20Object%20Reference))
  (|CallParentFunction OtherActor) ; This node is disabled and will not be called.\nDrag off pins to build functionality.
)

(event EventTick
  (params (DeltaSeconds :type Float%20%28single-precision%29))
  (|CallParentFunction DeltaSeconds) ; This node is disabled and will not be called.\nDrag off pins to build functionality.
)

(fn ConstructionScript
  (|CallParentFunction))

(fn GetDropLocation
  (bind _returnvalue (Components|GetOwner))
  (return (+ (Transformation|GetActorLocation _returnvalue) (* (Math|Random|RandomUnitVectorinConeinDegrees (Transformation|GetActorForwardVector _returnvalue) 55.0) 1.2e+02))))