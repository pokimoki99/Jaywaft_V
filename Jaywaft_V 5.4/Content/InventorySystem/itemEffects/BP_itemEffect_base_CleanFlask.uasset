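; Inventory item effect actor for the Clean Flask that restores player health as soon as it spawns.
; BeginPlay calls the restoreHealth event, which casts player 0's pawn to BP_ThirdPersonCharacter and adds a fixed amount to Health, clamped to the maximum.
; The actor destroys itself after healing; at full health it only prints a debug message and stays in the world.
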(event Custom|restoreHealth
  (bind _asbp_third_person_character (Utilities|Casting|CastToBP_ThirdPersonCharacter (Game|GetPlayerCharacter 0)))
  (if (< (Variables|/Game/ThirdPerson/Blueprints/BP_ThirdPersonCharacter.BP_ThirdPersonCharacter_C|Gethealth _asbp_third_person_character) 1e+02)
    (Variables|/Game/ThirdPerson/Blueprints/BP_ThirdPersonCharacter.BP_ThirdPersonCharacter_C|Sethealth _asbp_third_person_character (Math|Float|Clamp(Float) (+ (Variables|/Game/ThirdPerson/Blueprints/BP_ThirdPersonCharacter.BP_ThirdPersonCharacter_C|Gethealth _asbp_third_person_character) 2e+01) 0.0 1e+02))
    (Actor|DestroyActor)
    (else
      (Development|PrintString "health full"))))

(event EventBeginPlay
  (|CallParentFunction)
  (Development|PrintString "restore health")
  (CallFunction|RestoreHealth))

(event Collision|EventActorBeginOverlap
  (params (OtherActor :type Actor%20Object%20Reference)))

(event EventTick
  (params (DeltaSeconds :type Float%20%28single-precision%29))
  (|CallParentFunction DeltaSeconds) ; This node is disabled and will not be called.\nDrag off pins to build functionality.
)

(fn ConstructionScript
  (|CallParentFunction))