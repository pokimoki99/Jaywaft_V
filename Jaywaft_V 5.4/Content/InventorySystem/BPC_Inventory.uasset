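; Inventory component that gives its owner item slots with stacking, splitting, transfer between inventories, use and drop, plus world interaction.
; A looping timer sphere-traces for a target and updates a prompt widget; the interact input messages that target.
; DT_itemData rows supply stack limits, sounds and classes spawned in front of the owner on use or drop.
; Splits, transfers, use and removal fire an inventory-updated event.
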(event Custom|CreateInteractMessage
  (bind _returnvalue (UserInterface|CreateWidget "/Game/InventorySystem/UI/WB_interactPrompt.WB_interactPrompt_C"))
  (bind _output_get (Variables|Default|SetWB_InteractMessage _returnvalue))
  (UserInterface|Viewport|AddtoViewport _output_get 0))

(event Custom|beginInteraction
  (Utilities|Time|SetTimerbyEvent (delegate Custom|updateInteraction) 0.2 true))

(event Custom|updateInteraction
  (CallFunction|Interaction))

(event Custom|updateInventory
  (Default|CallOnInventoryUpdated))

(event Input|EnhancedActionEvents|EnhancedInputActionIA_Interact
  (params (ActionValue :type Boolean) (ElapsedSeconds :type Float%20%28double-precision%29) (TriggeredSeconds :type Float%20%28double-precision%29) (InputAction :type Input%20Action%20Object%20Reference :default "/Game/Input/IA_Interact.IA_Interact"))
  (bind _returnvalue (Game|GetPlayerCharacter 0))
  (bind _asbp_third_person_character (Utilities|Casting|CastToBP_ThirdPersonCharacter _returnvalue))
  (:Started
    (bind _targetactor (Variables|Default|GettargetActor)
      (:then
        (Utilities|IsValid (Actor|GetComponentbyClass _targetactor "/Game/InventorySystem/BPC_itemData.BPC_itemData_C")
          (:Is%20Valid
            (Class|BPIInteract|Interact(Message) (Actor|GetComponentbyClass _targetactor "/Game/InventorySystem/BPC_itemData.BPC_itemData_C") _asbp_third_person_character))
          (:Is%20Not%20Valid
            (Class|BPIInteract|Interact(Message) (Variables|Default|GettargetActor) _asbp_third_person_character)
            (Class|BPIInteract|OnInteract(Message) (Variables|Default|GettargetActor)))))
      (:else))))

(event EventBeginPlay
  (Utilities|Array|Resize (Variables|Default|GetitemSlots) (Variables|Default|GetInventorySize)))

(fn PrintInventory
  (for (_array_element _array_index) (Variables|Default|GetitemSlots)
    (Development|PrintString (Utilities|String|Append (Utilities|String|ToString(Integer) _array_index) ":" (Utilities|String|ToString(Name) (.itemID (Utilities|Struct|BreakS_itemSlot _array_element))) "=" (Utilities|String|ToString(Integer) (.itemQuantity (Utilities|Struct|BreakS_itemSlot _array_element)))))))

(fn Interaction
  (bind _returnvalue (Components|GetOwner))
  (bind _returnvalue_2 (Transformation|GetActorLocation _returnvalue))
  (bind (_outhit _returnvalue_3) (Collision|SphereTraceByChannel _returnvalue_2 _returnvalue_2 (Variables|Default|GetinteractionRadius) "TraceTypeQuery3" false (Utilities|Array|MakeArray (Components|GetOwner)) "None"))
  (if _returnvalue_3
    (if (!= (.HitActor (Collision|BreakHitResult _outhit)) (Variables|Default|GettargetActor))
      (bind _output_get (Variables|Default|SettargetActor (.HitActor (Collision|BreakHitResult _outhit))))
      (bind _prompt (Class|BPIInteract|FocusTarget(Message) _output_get))
      (Default|SetInteractableMessage (Variables|Default|GetWB_InteractMessage) _prompt))
    (else
      (Variables|Default|SettargetActor 0)
      (Default|SetInteractableMessage (Variables|Default|GetWB_InteractMessage)))))

(fn PickUp
  (params (itemID :type Name) (itemQuantity :type Integer))
  (bind (_success _index) (CallFunction|AnySlotAvailable))
  (bind _output_get (LocalVariables|Setlocal_itemQuantity itemQuantity))
  (while (and (> _output_get 0) (not (LocalVariables|Getlocal_isFull)))
    (bind (_success_2 _index_2) (CallFunction|FindSlot itemID))
    (if _success_2
      (CallFunction|AddtoStack _index_2 1)
      (Math|Integer|DecrementInt (LocalVariables|Getlocal_itemQuantity)
        (:%20%20
          (Development|PrintString "added to stack")
          (return true 0)))
      (elif _success
        (CallFunction|CreateNewStack itemID 1 _index)
        (Math|Integer|DecrementInt (LocalVariables|Getlocal_itemQuantity)
          (:%20%20
            (Development|PrintString "created new stack")
            (return true 0)))
        (else
          (LocalVariables|Setlocal_isFull true)))))
  (return (not (LocalVariables|Getlocal_isFull)) (LocalVariables|Getlocal_itemQuantity)))

(fn FindSlot
  (params (itemID :type Name))
  (for (_array_element _array_index) (Variables|Default|GetitemSlots)
    (if (and (== itemID (.itemID (Utilities|Struct|BreakS_itemSlot _array_element))) (< (.itemQuantity (Utilities|Struct|BreakS_itemSlot _array_element)) (CallFunction|GetMaxStackSize itemID)))
      (return true _array_index)))
  (return false -1))

(fn GetMaxStackSize
  (params (itemID :type Name))
  (bind _returnvalue (Utilities|GetDataTableRow "/Game/InventorySystem/itemData/DT_itemData.DT_itemData" itemID)
    (:then
      (return (.SlotQuantity (Utilities|Struct|BreakS_itemData _returnvalue))))))

(fn AddtoStack
  (params (Index :type Integer) (itemQuantity :type Integer))
  (bind _itemslots (Variables|Default|GetitemSlots))
  (bind _output (Utilities|Array|Get(acopy) _itemslots Index))
  (Utilities|Array|SetArrayElem _itemslots Index (Utilities|Struct|MakeS_itemSlot (.itemid _output) (+ (.itemquantity _output) itemQuantity))))

(fn AnySlotAvailable
  (for (_array_element _array_index) (Variables|Default|GetitemSlots)
    (if (== (Utilities|Struct|BreakS_itemSlot _array_element) 0)
      (return true _array_index)))
  (return false -1))

(fn CreateNewStack
  (params (itemID :type Name) (itemQuantity :type Integer) (Index :type Integer))
  (Utilities|Array|SetArrayElem (Variables|Default|GetitemSlots) Index (Utilities|Struct|MakeS_itemSlot itemID itemQuantity)))

(fn SplitStack
  (params (index :type Integer))
  (bind (_success _index) (CallFunction|AnySlotAvailable))
  (bind _itemslots (Variables|Default|GetitemSlots))
  (bind _output (Utilities|Array|Get(acopy) _itemslots index))
  (LocalVariables|Setlocal_itemID (.itemid _output))
  (LocalVariables|Setlocal_itemQuantity (.itemquantity _output))
  (Utilities|FlowControl|Sequence
    (:then_0
      (if (not (== (LocalVariables|Getlocal_itemQuantity) 1))
        (if _success
          (LocalVariables|Setlocal_splitQuantity (/ (LocalVariables|Getlocal_itemQuantity) 2))
          (Utilities|Array|SetArrayElem (Variables|Default|GetitemSlots) _index (Utilities|Struct|MakeS_itemSlot (LocalVariables|Getlocal_itemID) (LocalVariables|Getlocal_splitQuantity)))
          (Utilities|Array|SetArrayElem (Variables|Default|GetitemSlots) index (Utilities|Struct|MakeS_itemSlot (LocalVariables|Getlocal_itemID) (- (LocalVariables|Getlocal_itemQuantity) (LocalVariables|Getlocal_splitQuantity)))))))
    (:then_1
      (bind _returnvalue (Utilities|GetDataTableRow "/Game/InventorySystem/itemData/DT_itemData.DT_itemData" (LocalVariables|Getlocal_itemID))
        (:then
          (Audio|PlaySoundatLocation (Utilities|Struct|BreakS_itemSFX (.SFX (Utilities|Struct|BreakS_itemData _returnvalue))) (Transformation|GetActorLocation (Components|GetOwner)) "0, 0, 0" 1.0 1.0 0.0 0 0 0 0)
          (CallFunction|UpdateInventory))))))

(fn UseItem
  (params (index :type Integer))
  (bind _itemslots (Variables|Default|GetitemSlots))
  (bind _output (Utilities|Array|Get(acopy) _itemslots index))
  (LocalVariables|Setlocal_itemID (.itemid _output))
  (LocalVariables|Setlocal_itemQuantity (.itemquantity _output))
  (Utilities|FlowControl|Sequence
    (:then_0
      (if (== (LocalVariables|Getlocal_itemQuantity) 1)
        (Utilities|Array|SetArrayElem (Variables|Default|GetitemSlots) index (Utilities|Struct|MakeS_itemSlot "None" 0))
        (else
          (CallFunction|UpdateStack index 1)))
      (Game|SpawnActorfromClass (Utilities|Struct|BreakS_itemData (CallFunction|GetItemData (LocalVariables|Getlocal_itemID))) (Math|Transform|MakeTransform (CallFunction|GetDropLocation) "0, 0, 0" "1.000000,1.000000,1.000000") "Undefined" "MultiplyWithRoot" 0 0))
    (:then_1
      (bind _returnvalue (Utilities|GetDataTableRow "/Game/InventorySystem/itemData/DT_itemData.DT_itemData" (LocalVariables|Getlocal_itemID))
        (:then
          (Audio|PlaySoundatLocation (Utilities|Struct|BreakS_itemSFX (.SFX (Utilities|Struct|BreakS_itemData _returnvalue))) (Transformation|GetActorLocation (Components|GetOwner)) "0, 0, 0" 1.0 1.0 0.0 0 0 0 0)
          (CallFunction|UpdateInventory))))))

(fn UpdateStack
  (params (index :type Integer) (itemQuantity :type Integer))
  (bind _itemslots (Variables|Default|GetitemSlots))
  (bind _output (Utilities|Array|Get(acopy) _itemslots index))
  (Utilities|Struct|SetmembersinS_itemSlot _output (- (Utilities|Struct|BreakS_itemSlot _output) itemQuantity)))

(fn GetDropLocation
  (bind _returnvalue (Components|GetOwner))
  (return (+ (Transformation|GetActorLocation _returnvalue) (* (Math|Random|RandomUnitVectorinConeinDegrees (Transformation|GetActorForwardVector _returnvalue) 55.0) 1.2e+02))))

(fn GetItemData
  (params (itemID :type Name))
  (bind _returnvalue (Utilities|GetDataTableRow "/Game/InventorySystem/itemData/DT_itemData.DT_itemData" itemID)
    (:then
      (return _returnvalue))))

(fn TransferSlot
  (params (index :type Integer) (sourceIndex :type Integer) (sourceInventory :type BPC%20Inventory%20Object%20Reference))
  (bind _itemslots (Variables|Default|GetitemSlots))
  (bind _output (Utilities|Array|Get(acopy) _itemslots index))
  (Utilities|FlowControl|Sequence
    (:then_0
      (LocalVariables|Setlocal_sourceSlot (Utilities|Array|Get(acopy) (Variables|BPC_Inventory_C|GetitemSlots sourceInventory) sourceIndex))
      (if (== (Utilities|Struct|BreakS_itemSlot (LocalVariables|Getlocal_sourceSlot)) (Utilities|Struct|BreakS_itemSlot (Utilities|Array|Get(acopy) (Variables|Default|GetitemSlots) index)))
        (CallFunction|CreateNewStack sourceInventory (select (> (Math|Integer|Clamp(Integer) (- (+ (.itemQuantity (Utilities|Struct|BreakS_itemSlot (LocalVariables|Getlocal_sourceSlot))) (Utilities|Struct|BreakS_itemSlot (Utilities|Array|Get(acopy) (Variables|Default|GetitemSlots) index))) (CallFunction|GetMaxStackSize (.itemID (Utilities|Struct|BreakS_itemSlot (LocalVariables|Getlocal_sourceSlot))))) 0 (CallFunction|GetMaxStackSize (.itemID (Utilities|Struct|BreakS_itemSlot (LocalVariables|Getlocal_sourceSlot))))) 0) (Utilities|Struct|BreakS_itemSlot (LocalVariables|Getlocal_sourceSlot)) "None") (Math|Integer|Clamp(Integer) (- (+ (.itemQuantity (Utilities|Struct|BreakS_itemSlot (LocalVariables|Getlocal_sourceSlot))) (Utilities|Struct|BreakS_itemSlot (Utilities|Array|Get(acopy) (Variables|Default|GetitemSlots) index))) (CallFunction|GetMaxStackSize (.itemID (Utilities|Struct|BreakS_itemSlot (LocalVariables|Getlocal_sourceSlot))))) 0 (CallFunction|GetMaxStackSize (.itemID (Utilities|Struct|BreakS_itemSlot (LocalVariables|Getlocal_sourceSlot))))) sourceIndex)
        (CallFunction|CreateNewStack (Utilities|Struct|BreakS_itemSlot (LocalVariables|Getlocal_sourceSlot)) (Math|Integer|Clamp(Integer) (+ (.itemQuantity (Utilities|Struct|BreakS_itemSlot (LocalVariables|Getlocal_sourceSlot))) (Utilities|Struct|BreakS_itemSlot (Utilities|Array|Get(acopy) (Variables|Default|GetitemSlots) index))) 0 (CallFunction|GetMaxStackSize (.itemID (Utilities|Struct|BreakS_itemSlot (LocalVariables|Getlocal_sourceSlot))))) index)
        (else
          (CallFunction|CreateNewStack sourceInventory (.itemid _output) (.itemquantity _output) sourceIndex)
          (CallFunction|CreateNewStack (.itemID (Utilities|Struct|BreakS_itemSlot (LocalVariables|Getlocal_sourceSlot))) (.itemQuantity (Utilities|Struct|BreakS_itemSlot (LocalVariables|Getlocal_sourceSlot))) index))))
    (:then_1
      (bind _returnvalue (Utilities|GetDataTableRow "/Game/InventorySystem/itemData/DT_itemData.DT_itemData" (Utilities|Struct|BreakS_itemSlot (Utilities|Array|Get(acopy) (Variables|Default|GetitemSlots) index)))
        (:then
          (Audio|PlaySoundatLocation (Utilities|Struct|BreakS_itemSFX (.SFX (Utilities|Struct|BreakS_itemData _returnvalue))) (Transformation|GetActorLocation (Components|GetOwner)) "0, 0, 0" 1.0 1.0 0.0 0 0 0 0)
          (CallFunction|UpdateInventory)
          (CallFunction|UpdateInventory sourceInventory))))))

(fn RemovefromInventory
  (params (index :type Integer) (dropQuantity :type Integer))
  (bind _itemslots (Variables|Default|GetitemSlots))
  (bind _output (Utilities|Array|Get(acopy) _itemslots index))
  (LocalVariables|Setlocal_itemID (.itemid _output))
  (LocalVariables|Setlocal_itemQuantity (.itemquantity _output))
  (Utilities|FlowControl|Sequence
    (:then_0
      (if (== dropQuantity (LocalVariables|Getlocal_itemQuantity))
        (Utilities|Array|SetArrayElem (Variables|Default|GetitemSlots) index (Utilities|Struct|MakeS_itemSlot "None" 0))
        (CallFunction|DropfromInventory (LocalVariables|Getlocal_itemID) dropQuantity)
        (elif (== (LocalVariables|Getlocal_itemQuantity) 1)
          (Utilities|Array|SetArrayElem (Variables|Default|GetitemSlots) index (Utilities|Struct|MakeS_itemSlot "None" 0))
          (CallFunction|DropfromInventory (LocalVariables|Getlocal_itemID) 1)
          (else
            (CallFunction|UpdateStack index dropQuantity)
            (CallFunction|DropfromInventory (LocalVariables|Getlocal_itemID) dropQuantity)))))
    (:then_1
      (CallFunction|UpdateInventory))))

(fn DropfromInventory
  (params (itemID :type Name) (itemQuantity :type Integer))
  (bind _itemdata (CallFunction|GetItemData itemID))
  (bind _location (CallFunction|GetDropLocation))
  (bind (_class _sfx) (Utilities|Struct|BreakS_itemData _itemdata))
  (for _index (range 0 (- itemQuantity 1))
    (Game|SpawnActorfromClass _class (Math|Transform|MakeTransform _location "0, 0, 0" "1.000000,1.000000,1.000000") "Undefined" "MultiplyWithRoot" 0 0)
    (Audio|PlaySoundatLocation (Utilities|Struct|BreakS_itemSFX _sfx) _location "0, 0, 0" 1.0 1.0 0.0 0 0 0 0)))