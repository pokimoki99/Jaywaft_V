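; Inventory component that stores item stacks in a fixed-size slot array and detects nearby interactables for its owner.
; A looping timer sphere-traces around the owner and shows the focused actor's message in a prompt widget.
; PickUp adds to a matching stack or the first empty slot, returning after one unit.
; Stack limits come from DT_itemData, but FindSlot's comparison is inverted, matching only stacks above the limit.
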(event Custom|CreateInteractMessage
  (bind _returnvalue (UserInterface|CreateWidget "/Game/InventorySystem/UI/WB_interactPrompt.WB_interactPrompt_C"))
  (bind _output_get (Variables|Default|SetWB_InteractMessage _returnvalue))
  (UserInterface|Viewport|AddtoViewport _output_get 0))

(event Custom|beginInteraction
  (Utilities|Time|SetTimerbyEvent (delegate Custom|updateInteraction) 0.2 true))

(event Custom|updateInteraction
  (CallFunction|Interaction))

(event EventBeginPlay
  (Utilities|Array|Resize (Variables|Default|GetitemSlots) (Variables|Default|GetInventorySize)))

(fn PrintInventory
  (for (_array_element _array_index) (Variables|Default|GetitemSlots)
    (Development|PrintString (Utilities|String|Append (Utilities|String|ToString(Integer) _array_index) ":" (Utilities|String|ToString(Name) (.itemID (Utilities|Struct|BreakS_itemSlot _array_element))) "=" (Utilities|String|ToString(Integer) (.itemQuantity (Utilities|Struct|BreakS_itemSlot _array_element)))))))

(fn Interaction
  (bind _returnvalue (Components|GetOwner))
  (bind _returnvalue_2 (Transformation|GetActorLocation _returnvalue))
  (bind (_outhit _returnvalue_3) (Collision|SphereTraceByChannel _returnvalue_2 _returnvalue_2 (Variables|Default|GetinteractionRadius) "TraceTypeQuery3" false (Utilities|Array|MakeArray (Components|GetOwner)) "None"))
  (if _returnvalue_3
    (if (!= (.HitActor (Collision|BreakHitResult _outhit)) (Variables|Default|GettargetActor))
      (bind _output_get (Variables|Default|SettargetActor (.HitActor (Collision|BreakHitResult _outhit))))
      (bind _prompt (Class|BPIInteract|FocusTarget(Message) _output_get))
      (Default|SetInteractableMessage (Variables|Default|GetWB_InteractMessage) _prompt))
    (else
      (Variables|Default|SettargetActor 0)
      (Default|SetInteractableMessage (Variables|Default|GetWB_InteractMessage)))))

(fn PickUp
  (params (itemID :type Name) (itemQuantity :type Integer))
  (bind (_success _index) (CallFunction|AnySlotAvailable))
  (bind _output_get (LocalVariables|Setlocal_itemQuantity itemQuantity))
  (while (and (> _output_get 0) (not (LocalVariables|Getlocal_isFull)))
    (bind (_success_2 _index_2) (CallFunction|FindSlot itemID))
    (if _success_2
      (CallFunction|AddtoStack _index_2 1)
      (Math|Integer|DecrementInt (LocalVariables|Getlocal_itemQuantity)
        (:%20%20
          (return true 0)))
      (elif _success
        (CallFunction|CreateNewStack itemID 1 _index)
        (Math|Integer|DecrementInt (LocalVariables|Getlocal_itemQuantity)
          (:%20%20
            (return true 0)))
        (else
          (LocalVariables|Setlocal_isFull true)))))
  (return (not (LocalVariables|Getlocal_isFull)) (LocalVariables|Getlocal_itemQuantity)))

(fn FindSlot
  (params (itemID :type Name))
  (for (_array_element _array_index) (Variables|Default|GetitemSlots)
    (if (and (== itemID (.itemID (Utilities|Struct|BreakS_itemSlot _array_element))) (< (CallFunction|GetMaxStackSize itemID) (.itemQuantity (Utilities|Struct|BreakS_itemSlot _array_element))))
      (return true _array_index)))
  (return false -1))

(fn GetMaxStackSize
  (params (itemID :type Name))
  (bind _returnvalue (Utilities|GetDataTableRow "/Game/InventorySystem/itemData/DT_itemData.DT_itemData" itemID)
    (:then
      (return (.SlotQuantity (Utilities|Struct|BreakS_itemData _returnvalue))))))

(fn AddtoStack
  (params (Index :type Integer) (itemQuantity :type Integer))
  (bind _itemslots (Variables|Default|GetitemSlots))
  (bind _output (Utilities|Array|Get(acopy) _itemslots Index))
  (Utilities|Array|SetArrayElem _itemslots Index (Utilities|Struct|MakeS_itemSlot (.itemid _output) (+ (.itemquantity _output) itemQuantity))))

(fn AnySlotAvailable
  (for (_array_element _array_index) (Variables|Default|GetitemSlots)
    (if (== (Utilities|Struct|BreakS_itemSlot _array_element) 0)
      (return true _array_index)))
  (return false -1))

(fn CreateNewStack
  (params (itemID :type Name) (itemQuantity :type Integer) (Index :type Integer))
  (Utilities|Array|SetArrayElem (Variables|Default|GetitemSlots) Index (Utilities|Struct|MakeS_itemSlot itemID itemQuantity)))