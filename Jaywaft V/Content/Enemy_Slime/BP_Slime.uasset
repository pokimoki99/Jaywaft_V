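; BP_Slime is an enemy slime pawn that chases the player character and fires slime projectiles at it.
; When PawnSensing sees a BP_ThirdPersonCharacter, it starts an AI move toward it, turns to face it and, if off cooldown, spawns a BP_SlimeAttack.
; The projectile is launched by a forward impulse with upward lift, and a boolean with a delay throttles firing.
; Any damage reduces its health, and it is destroyed at zero.
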(event OnSeePawn(PawnSensing)
  (params (Pawn :type Pawn%20Object%20Reference))
  (bind _asbp_third_person_character (Utilities|Casting|CastToBP_ThirdPersonCharacter Pawn))
  (AI|AIMoveTo self "0, 0, 0" _asbp_third_person_character 5.0 false
    (:then
      (Utilities|FlowControl|Sequence
        (:then_0
          (Transformation|SetActorRotation (Math|Rotator|FindLookatRotation (Transformation|GetActorLocation) (Transformation|GetActorLocation _asbp_third_person_character))))
        (:then_1
          (if (Variables|Default|GetSpawnSlimeProjectile)
            (bind _returnvalue (Game|SpawnActorfromClass "/Game/Enemy_Slime/BP_SlimeAttack.BP_SlimeAttack_C" (Transformation|GetWorldTransform (Variables|Default|GetSpawnProjectile)) "Undefined" "MultiplyWithRoot" 0 0))
            (Physics|AddImpulse (Variables|/Game/Enemy_Slime/BP_SlimeAttack.BP_SlimeAttack_C|GetSphere_replace _returnvalue) (+ (* (Math|Vector|GetForwardVector (Variables|Default|GetSlime)) (Variables|Default|GetShootImpluse)) "0.000000,0.000000,100.000000") "None" true)
            (Variables|Default|SetSpawnSlimeProjectile false)
            (Utilities|FlowControl|Delay 5.0)
            (Variables|Default|SetSpawnSlimeProjectile true)))))
    (:OnSuccess
      (Development|PrintString "working"))
    (:OnFail
      (Development|PrintString "fail"))))

(event EventBeginPlay)

(event Collision|EventActorBeginOverlap
  (params (OtherActor :type Actor%20Object%20Reference)))

(event EventTick
  (params (DeltaSeconds :type Float%20%28single-precision%29)))

(event Game|Damage|EventAnyDamage
  (params (Damage :type Float%20%28single-precision%29) (DamageType :type Damage%20Type%20Object%20Reference) (InstigatedBy :type Controller%20Object%20Reference) (DamageCauser :type Actor%20Object%20Reference))
  ;[1 1 1] Damage
  (Variables|Default|SetEnemy_Health (- (Variables|Default|GetEnemy_Health) Damage))
  (if (<= (Variables|Default|GetEnemy_Health) 0.0)
    (Actor|DestroyActor)))

(fn ConstructionScript)