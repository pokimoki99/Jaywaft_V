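; BP_throwable is a thrown flask whose look and hit effect depend on a quest number.
; CheckThrowable stores the quest number and shows the flask body at quest one, the clean label mesh above one, or neither.
; On hit, it destroys a slime if the quest is above one, or otherwise tells a movable obstacle to move.
; Either successful hit plays the splash effect, then destroys the flask after a short delay.
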(event OnComponentHit(flaskCollision)
  (params (HitComponent :type Primitive%20Component%20Object%20Reference) (OtherActor :type Actor%20Object%20Reference) (OtherComp :type Primitive%20Component%20Object%20Reference) (NormalImpulse :type Vector :default "0, 0, 0") (Hit :type Hit%20Result%20Structure%20%28by%20ref%29))
  (if (> (Variables|Default|GetQuest%20Num) 1)
    (bind _asbp_slime (Utilities|Casting|CastToBP_Slime OtherActor)
      (:then
        (CallFunction|VFX)
        (Actor|DestroyActor _asbp_slime))
      (:CastFailed
        (bind _asmovable_obstacle (Utilities|Casting|CastTomovableObstacle OtherActor :!label _label))
        (Default|MoveObstacle _asmovable_obstacle)
        (CallFunction|VFX)))
    (else
      (goto _label))))

(event Custom|VFX
  (Components|Activation|Activate (Variables|Default|GetSplashSFX) false)
  (Utilities|FlowControl|Delay 0.2)
  (Actor|DestroyActor))

(event EventBeginPlay
  (Components|Activation|Deactivate (Variables|Default|GetSplashSFX)))

(event Collision|EventActorBeginOverlap
  (params (OtherActor :type Actor%20Object%20Reference)))

(event EventTick
  (params (DeltaSeconds :type Float%20%28single-precision%29)))

(fn ConstructionScript)

(fn CheckThrowable
  (params (QuestNum :type Integer))
  (bind _clean_flask_lable_low (Variables|Default|GetClean_Flask_Lable_low))
  (Variables|Default|SetQuest%20Num QuestNum)
  (if (== QuestNum 1)
    (Rendering|SetVisibility (Variables|Default|GetFlask_Flask_Body_low) true true)
    (else
      (if (> QuestNum 1)
        (Rendering|SetVisibility _clean_flask_lable_low true true)
        (else
          (Rendering|SetVisibility _clean_flask_lable_low false true)))
      (Rendering|SetVisibility (Variables|Default|GetFlask_Flask_Body_low) false true)))
  (return))