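; BPC_itemData is an actor component that makes its owner a pickup for the inventory system, carrying an item row reference and quantity.
; On Interact it asks the interactor's inventory component to pick up that item and quantity.
; On success it looks up the item's row in DT_itemData, plays its pickup sound at the owner's location and destroys the owner.
; FocusTarget returns an empty string.
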(event EventBeginPlay)

(event EventTick
  (params (DeltaSeconds :type Float%20%28single-precision%29)))

(event EventInteract
  (params (Interactor :type BP%20Third%20Person%20Character%20Object%20Reference))
  (bind _bpc_inventory (Variables|/Game/ThirdPerson/Blueprints/BP_ThirdPersonCharacter.BP_ThirdPersonCharacter_C|GetBPC_Inventory Interactor)
    (:then
      (bind _success (Default|PickUp _bpc_inventory (Utilities|Struct|BreakDataTableRowHandle (Variables|Default|GetitemID)) (Variables|Default|GetitemQuantity)))
      (if _success
        (bind _returnvalue (Utilities|GetDataTableRow "/Game/InventorySystem/itemData/DT_itemData.DT_itemData" (.RowName (Utilities|Struct|BreakDataTableRowHandle (Variables|Default|GetitemID))))
          (:then
            (Audio|PlaySoundatLocation (Utilities|Struct|BreakS_itemSFX (.SFX (Utilities|Struct|BreakS_itemData _returnvalue))) (Transformation|GetActorLocation (Components|GetOwner)) "0, 0, 0" 1.0 1.0 0.0 0 0 0 0)
            (Actor|DestroyActor (Components|GetOwner))))))
    (:else)))

(fn FocusTarget
  (return ""))