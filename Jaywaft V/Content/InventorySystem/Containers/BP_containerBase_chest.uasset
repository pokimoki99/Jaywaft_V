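; Chest variant of the inventory container base that opens and closes when interacted with or updated.
; Each trigger toggles IsOpen, plays the matching open or close sound at the chest's location, and plays or reverses a timeline.
; The timeline rolls the second mesh, likely the lid, between closed and 120 degrees open.
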(event EventBeginPlay
  (|CallParentFunction) ; This node is disabled and will not be called.\nDrag off pins to build functionality.
)

(event EventOnInteract
  (bind _returnvalue (Transformation|GetActorLocation))
  (bind _containersfx (Variables|Default|GetcontainerSFX))
  (bind (_open _close) (Utilities|Struct|BreakS_containerSFX _containersfx))
  (if (not (Variables|Default|GetisOpen))
    (Variables|Default|SetisOpen true)
    (Audio|PlaySoundatLocation _open _returnvalue "0, 0, 0" 1.0 1.0 0.0 0 0 0 0)
    (bind _contrainertrack (Timeline|containerTimeline Play)
      (:Update
        (Transformation|SetRelativeRotation (Variables|Default|GetsecondMesh) (Math|Rotator|MakeRotator (Math|Float|Lerp 0.0 -1.2e+02 _contrainertrack) 0.0 0.0) false false)))
    (else
      (Variables|Default|SetisOpen false)
      (Audio|PlaySoundatLocation _close _returnvalue "0, 0, 0" 1.0 1.0 0.0 0 0 0 0)
      (Timeline|containerTimeline Reverse))))

(event EventUpdateContainer
  (bind _returnvalue (Transformation|GetActorLocation))
  (bind _containersfx (Variables|Default|GetcontainerSFX))
  (bind (_open _close) (Utilities|Struct|BreakS_containerSFX _containersfx))
  (if (not (Variables|Default|GetisOpen))
    (Variables|Default|SetisOpen true)
    (Audio|PlaySoundatLocation _open _returnvalue "0, 0, 0" 1.0 1.0 0.0 0 0 0 0)
    (bind _contrainertrack (Timeline|containerTimeline Play)
      (:Update
        (Transformation|SetRelativeRotation (Variables|Default|GetsecondMesh) (Math|Rotator|MakeRotator (Math|Float|Lerp 0.0 -1.2e+02 _contrainertrack) 0.0 0.0) false false)))
    (else
      (Variables|Default|SetisOpen false)
      (Audio|PlaySoundatLocation _close _returnvalue "0, 0, 0" 1.0 1.0 0.0 0 0 0 0)
      (Timeline|containerTimeline Reverse))))

(fn ConstructionScript
  (|CallParentFunction))