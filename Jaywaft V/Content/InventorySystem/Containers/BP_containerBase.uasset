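; Base Blueprint for searchable inventory containers that the player can open through interaction.
; On BeginPlay it copies its configured content into its BPCInventory component and resizes the slots to the container size.
; Interact has the local player's HUD create a container display for that inventory and binds to its closed event.
; FocusTarget supplies a "Search" prompt with the container's name, while updateContainer is an empty event.
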(event Custom|updateContainer)

(event EventBeginPlay
  (bind _bpc_inventory (Variables|Default|GetBPC_Inventory))
  (Variables|/Game/InventorySystem/BPC_Inventory.BPC_Inventory_C|SetitemSlots _bpc_inventory (Variables|Default|GetcontainerContent))
  (Utilities|Array|Resize (Variables|/Game/InventorySystem/BPC_Inventory.BPC_Inventory_C|GetitemSlots _bpc_inventory) (Variables|Default|GetcontainerSize)))

(event EventInteract
  (params (Interactor :type BP%20Third%20Person%20Character%20Object%20Reference))
  (bind _asbp_pcontroller (Utilities|Casting|CastToBP_PController (Game|GetPlayerController 0)))
  (bind _returnvalue (Default|CreateContainerDisplay (Variables|/Game/ThirdPerson/Blueprints/BP_PController.BP_PController_C|GetWB_playerHUD _asbp_pcontroller) (Variables|Default|GetBPC_Inventory)))
  (EventDispatchers|BindEventtoOnContainerClosed _returnvalue (EventDispatchers|CreateEvent :!event Custom|updateContainer)))

(fn ConstructionScript)

(fn FocusTarget
  (return (Utilities|Text|FormatText "Search {Container}" (Variables|Default|GetcontainerName))))