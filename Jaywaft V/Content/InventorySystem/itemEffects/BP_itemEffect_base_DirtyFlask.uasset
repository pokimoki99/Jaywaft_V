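; Inventory item effect actor for the Dirty Flask that damages the player as soon as it spawns.
; BeginPlay calls the removeHealth event, which casts the first player character to BP_ThirdPersonCharacter and directly lowers its clamped Health by a fixed amount.
; The actor destroys itself after applying the damage; if Health is already zero, it only prints a message and stays in the world.
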(event Custom|removeHealth
  (bind _asbp_third_person_character (Utilities|Casting|CastToBP_ThirdPersonCharacter (Game|GetPlayerCharacter 0)))
  (if (> (Variables|/Game/ThirdPerson/Blueprints/BP_ThirdPersonCharacter.BP_ThirdPersonCharacter_C|Gethealth _asbp_third_person_character) 0.0)
    (Variables|/Game/ThirdPerson/Blueprints/BP_ThirdPersonCharacter.BP_ThirdPersonCharacter_C|Sethealth _asbp_third_person_character (Math|Float|Clamp(Float) (- (Variables|/Game/ThirdPerson/Blueprints/BP_ThirdPersonCharacter.BP_ThirdPersonCharacter_C|Gethealth _asbp_third_person_character) 2e+01) 0.0 1e+02))
    (Actor|DestroyActor)
    (else
      (Development|PrintString "health at 0"))))

(event EventBeginPlay
  (|CallParentFunction)
  (Development|PrintString "remove health")
  (CallFunction|RemoveHealth))

(event Collision|EventActorBeginOverlap
  (params (OtherActor :type Actor%20Object%20Reference)))

(event EventTick
  (params (DeltaSeconds :type Float%20%28single-precision%29))
  (|CallParentFunction DeltaSeconds) ; This node is disabled and will not be called.\nDrag off pins to build functionality.
)

(fn ConstructionScript
  (|CallParentFunction))